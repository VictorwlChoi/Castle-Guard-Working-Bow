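; BP_Arrow is an arrow projectile actor in the Vive content, with its ProjectileMovement driving the static mesh.
; Releasing the Fire input attaches a trail emitter to the Scene component.
; While InFlight, which this graph never sets true, Tick applies a small constant local rotation and clears the flag once velocity reaches zero.
; Hit and Enemy-tag overlap handlers do nothing, as the emitter, debug and destroy nodes are disconnected.
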(event EventActorBeginOverlap
  (params (OtherActor :type Actor%20Object%20Reference))
  (if (Actor|ActorHasTag OtherActor "Enemy")
    _))

(event EventTick
  (params (DeltaSeconds :type Float%20%28single-precision%29))
  (if (Variables|Default|GetInFlight)
    (Variables|Default|SetInFlight (Math|Vector|NotEqual(Vector) (Variables|/Script/Engine.MovementComponent|GetVelocity (Variables|Default|GetProjectileMovement)) "0, 0, 0" 0.0001))
    (Transformation|AddActorLocalRotation "-0.500000, 0, 0" false false)))

(event Collision|EventHit
  (params (MyComp :type Primitive%20Component%20Object%20Reference) (Other :type Actor%20Object%20Reference) (OtherComp :type Primitive%20Component%20Object%20Reference) (bSelfMoved :type Boolean) (HitLocation :type Vector) (HitNormal :type Vector :default "0, 0, 0") (NormalImpulse :type Vector :default "0, 0, 0") (Hit :type Hit%20Result%20Structure%20%28by%20ref%29)))

(event Input|ActionEvents|InputActionFire
  (params (Key :type Key%20Structure :default "AnyKey"))
  (:Released
    (Effects|SpawnEmitterAttached "/Game/Particles/ArrowTrail.ArrowTrail" (Variables|Default|GetScene) "None" (Transformation|GetActorLocation) (Transformation|GetActorRotation))))

(fn ConstructionScript
  (Components|Movement|SetUpdatedComponent (Variables|Default|GetProjectileMovement) (Variables|Default|GetStaticMesh))
  (Variables|Default|SetInFlight false)
  (Variables|Default|SetHit false)
  (Variables|Default|SetChump "Chump"))