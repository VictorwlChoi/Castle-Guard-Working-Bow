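; AI catapult pawn that soldiers attach to and that then moves itself toward an attack position.
; The first two overlapping Soldier-tagged actors snap to the handle sockets on the Cube, and the first starts an AI move to FirstPos.
; While a handle is held and FirstPos.FinalLocation is true, Tick re-issues moves to FinalLocation, or to its NextPosition if taken.
; Capsule overlap with an AiAttackPosition_Catapult sets HasPosition, ending the Tick-driven moves.
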(event OnComponentBeginOverlap(CapsuleComponent)
  (params (OverlappedComponent :type Primitive%20Component%20Object%20Reference) (OtherActor :type Actor%20Object%20Reference) (OtherComp :type Primitive%20Component%20Object%20Reference) (OtherBodyIndex :type Integer) (bFromSweep :type Boolean) (SweepResult :type Hit%20Result%20Structure%20%28by%20ref%29))
  (Utilities|Casting|CastToAiAttackPosition_Catapult OtherActor)
  (Variables|Default|SetHasPosition true))

(event EventTick
  (params (DeltaSeconds :type Float%20%28single-precision%29))
  (if (Variables|Default|GetHandleBool1)
    (if (not (Variables|Default|GetHasPosition))
      (if (Variables|/Game/Vive/Blueprints/AI/AIStops_Catapult.AIStops_Catapult_C|GetFinalLocation (Variables|Default|GetFirstPos))
        (if (Variables|/Game/Vive/Blueprints/AI/AiAttackPosition_Catapult.AiAttackPosition_Catapult_C|GetPositionTaken (Variables|Default|GetFinalLocation))
          (AI|AIMoveTo self "0, 0, 0" (Variables|/Game/Vive/Blueprints/AI/AiAttackPosition_Catapult.AiAttackPosition_Catapult_C|GetNextPosition (Variables|Default|GetFinalLocation)) 5.0 true
            (:then
              (Variables|Default|SetFinalLocation (Variables|/Game/Vive/Blueprints/AI/AiAttackPosition_Catapult.AiAttackPosition_Catapult_C|GetNextPosition (Variables|Default|GetFinalLocation)))))
          (else
            (AI|AIMoveTo self "0, 0, 0" (Variables|Default|GetFinalLocation) 5.0 true)))))))

(event Collision|EventActorBeginOverlap
  (params (OtherActor :type Actor%20Object%20Reference))
  (bind _handlestring2 (Variables|Default|GetHandleString2))
  (bind _handlestring1 (Variables|Default|GetHandleString1))
  (if (Actor|ActorHasTag OtherActor "Soldier")
    (if (not (Variables|Default|GetHandleBool2))
      (if (Variables|Default|GetHandleBool1)
        (Variables|Default|SetHandleBool2 true)
        (Development|PrintString _handlestring2)
        (Transformation|AttachComponentToComponent OtherActor (Variables|Default|GetCube) (Utilities|String|StringToName _handlestring2) "SnapToTarget" "SnapToTarget" "KeepWorld" false)
        (else
          (Variables|Default|SetHandleBool1 true)
          (Development|PrintString _handlestring1)
          (Transformation|AttachComponentToComponent OtherActor (Variables|Default|GetCube) (Utilities|String|StringToName _handlestring1) "SnapToTarget" "SnapToTarget" "KeepWorld" false)
          (AI|AIMoveTo self (Transformation|GetActorLocation) (Variables|Default|GetFirstPos) 1e+01 false))))))

(event EventBeginPlay)

(fn ConstructionScript
  (Variables|Default|SetHandleBool1 false)
  (Variables|Default|SetHandleString1 "Handle1")
  (Variables|Default|SetHandleString2 "Handle2")
  (Variables|Default|SetHandleBool2 false))