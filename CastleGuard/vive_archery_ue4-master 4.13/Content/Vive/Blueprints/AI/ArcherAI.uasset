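; Archer AI pawn that walks to an attack position and is destroyed when hit by an Arrow-tagged actor.
; BeginPlay moves it to FirstStop; once that is the last station, Tick heads for AttackPos, following NextPosition links past taken spots.
; Overlapping an attack position, or a battering ram or catapult while its referenced HandleBool2 is false, sets HasPosition, which halts movement every tick.
; Overlaps also print debug strings.
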(event OnComponentBeginOverlap(CapsuleComponent)
  (params (OverlappedComponent :type Primitive%20Component%20Object%20Reference) (OtherActor :type Actor%20Object%20Reference) (OtherComp :type Primitive%20Component%20Object%20Reference) (OtherBodyIndex :type Integer) (bFromSweep :type Boolean) (SweepResult :type Hit%20Result%20Structure%20%28by%20ref%29))
  (Utilities|Casting|CastToAiAttackPosition OtherActor)
  (Variables|Default|SetHasPosition true))

(event Collision|EventHit
  (params (MyComp :type Primitive%20Component%20Object%20Reference) (Other :type Actor%20Object%20Reference) (OtherComp :type Primitive%20Component%20Object%20Reference) (bSelfMoved :type Boolean) (HitLocation :type Vector :default "0, 0, 0") (HitNormal :type Vector :default "0, 0, 0") (NormalImpulse :type Vector :default "0, 0, 0") (Hit :type Hit%20Result%20Structure%20%28by%20ref%29))
  (if (Actor|ActorHasTag Other "Arrow")
    (Actor|DestroyActor)))

(event EventTick
  (params (DeltaSeconds :type Float%20%28single-precision%29))
  (if (Variables|Default|GetHasPosition)
    (Components|Movement|StopMovementImmediately (Variables|Character|GetCharacterMovement))
    (elif (Variables|/Game/Vive/Blueprints/AI/AiStops_Soldier.AiStops_Soldier_C|GetLastStation? (Variables|Default|GetFirstStop))
      (if (Variables|/Game/Vive/Blueprints/AI/AiAttackPosition.AiAttackPosition_C|GetPositionTaken (Variables|Default|GetAttackPos))
        (AI|AIMoveTo self "0, 0, 0" (Variables|/Game/Vive/Blueprints/AI/AiAttackPosition.AiAttackPosition_C|GetNextPosition (Variables|Default|GetAttackPos)) 5.0 true
          (:then
            (Variables|Default|SetAttackPos (Variables|/Game/Vive/Blueprints/AI/AiAttackPosition.AiAttackPosition_C|GetNextPosition (Variables|Default|GetAttackPos)))))
        (else
          (AI|AIMoveTo self "0, 0, 0" (Variables|Default|GetAttackPos) 5.0 true))))))

(event EventBeginPlay
  (AI|AIMoveTo self "0, 0, 0" (Variables|Default|GetFirstStop) 1e+01 false))

(event Collision|EventActorBeginOverlap
  (params (OtherActor :type Actor%20Object%20Reference))
  (bind _returnvalue (Utilities|GetClass OtherActor))
  (Development|PrintString (Utilities|GetClassDisplayName _returnvalue))
  (if (Utilities|ClassIsChildOf _returnvalue "/Game/Vive/Blueprints/AI/VC_PrototypeBatteringRam.VC_PrototypeBatteringRam_C")
    (if (not (Variables|/Game/Vive/Blueprints/AI/VC_PrototypeBatteringRam.VC_PrototypeBatteringRam_C|GetHandleBool2 (Variables|Default|GetBatteringRam)))
      (Variables|Default|SetHasPosition true))
    (elif (Utilities|ClassIsChildOf _returnvalue "/Game/Vive/Blueprints/AI/Catapult.Catapult_C")
      (if (not (Variables|/Game/Vive/Blueprints/AI/Catapult.Catapult_C|GetHandleBool2 (Variables|Default|GetCatapult)))
        (Variables|Default|SetHasPosition true))
      (else
        (Development|PrintString "Hello")))))

(fn ConstructionScript)