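; BP_Arrow is the projectile arrow for the Vive bow, driven by a ProjectileMovement component acting on its static mesh.
; While InFlight, Tick rotates it slightly each frame and clears the flag once velocity reaches zero; nothing here sets that flag true.
; The Hit event attaches a particle effect to the mesh at the hit location.
; Overlap is empty, and the logic to destroy Enemy-tagged actors is disconnected.
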(event Collision|EventHit
  (params (MyComp :type Primitive%20Component%20Object%20Reference) (Other :type Actor%20Object%20Reference) (OtherComp :type Primitive%20Component%20Object%20Reference) (bSelfMoved :type Boolean) (HitLocation :type Vector) (HitNormal :type Vector :default "0, 0, 0") (NormalImpulse :type Vector :default "0, 0, 0") (Hit :type Hit%20Result%20Structure%20%28by%20ref%29))
  (bind _returnvalue (Effects|SpawnEmitterAttached "/Game/Particles/DefaultParticle.DefaultParticle" (Variables|Default|GetStaticMesh) "None" HitLocation "0, 0, 0" "KeepRelativeOffset" false)))

(event EventActorBeginOverlap
  (params (OtherActor :type Actor%20Object%20Reference)))

(event EventTick
  (params (DeltaSeconds :type Float%20%28single-precision%29))
  (if (Variables|Default|GetInFlight)
    (Variables|Default|SetInFlight (Math|Vector|NotEqual(Vector) (Variables|/Script/Engine.MovementComponent|GetVelocity (Variables|Default|GetProjectileMovement)) "0, 0, 0" 0.0001))
    (Transformation|AddActorLocalRotation "-0.500000,0.000000, 0" false false)))

(fn ConstructionScript
  (Components|Movement|SetUpdatedComponent (Variables|Default|GetProjectileMovement) (Variables|Default|GetStaticMesh))
  (Variables|Default|SetInFlight false)
  (Variables|Default|SetHit false)
  (Variables|Default|SetSocketFlame "Flame")
  (Variables|Default|SetSocketTrail "Trail")
  (if true
    _))