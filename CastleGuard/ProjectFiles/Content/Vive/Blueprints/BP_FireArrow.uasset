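; BP_FireArrow is a projectile arrow Blueprint, with flame and trail socket names set at construction.
; The construction script makes the static mesh the ProjectileMovement's updated component and clears the flight and hit flags.
; While InFlight is true, Tick applies a small local rotation and clears the flag once velocity reaches zero.
; The overlap event is empty; logic to destroy Enemy-tagged actors is disconnected.
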(event Collision|EventActorBeginOverlap
  (params (OtherActor :type Actor%20Object%20Reference)))

(event EventTick
  (params (DeltaSeconds :type Float%20%28single-precision%29))
  (if (Variables|Default|GetInFlight)
    (Variables|Default|SetInFlight (Math|Vector|NotEqual(Vector) (Variables|/Script/Engine.MovementComponent|GetVelocity (Variables|Default|GetProjectileMovement)) "0, 0, 0" 0.0001))
    (Transformation|AddActorLocalRotation "-0.500000,0.000000, 0" false false)))

(fn ConstructionScript
  (Components|Movement|SetUpdatedComponent (Variables|Default|GetProjectileMovement) (Variables|Default|GetStaticMesh))
  (Variables|Default|SetInFlight false)
  (Variables|Default|SetHit false)
  (Variables|Default|SetSocketFlame "Flame")
  (Variables|Default|SetSocketTrail "Trail")
  (if true
    _))