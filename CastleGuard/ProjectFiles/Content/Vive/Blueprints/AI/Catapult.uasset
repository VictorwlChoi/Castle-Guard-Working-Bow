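; AI catapult character that soldiers man and push to an attack position, and that fire arrows can burn down.
; Overlapping soldiers snap onto two handle sockets, raising its speed; once full it moves to FirstPos, then seeks a free FinalLocation, stopping on overlapping an attack position.
; Tick drives movement, burn damage, the player-facing health bar and destruction at zero health.
; Soldiers hitting its Cube get redirected to NextCatapult.
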(event OnComponentBeginOverlap(CapsuleComponent)
  (params (OverlappedComponent :type Primitive%20Component%20Object%20Reference) (OtherActor :type Actor%20Object%20Reference) (OtherComp :type Primitive%20Component%20Object%20Reference) (OtherBodyIndex :type Integer) (bFromSweep :type Boolean) (SweepResult :type Hit%20Result%20Structure%20%28by%20ref%29))
  ;[1 1 1] Moving AI
  (Utilities|Casting|CastToAiAttackPosition_Catapult OtherActor)
  (Variables|Default|SetHasPosition true))

(event OnComponentHit(Cube)
  (params (HitComponent :type Primitive%20Component%20Object%20Reference) (OtherActor :type Actor%20Object%20Reference) (OtherComp :type Primitive%20Component%20Object%20Reference) (NormalImpulse :type Vector :default "0, 0, 0") (Hit :type Hit%20Result%20Structure%20%28by%20ref%29))
  ;[1 1 1] Checking for someone manning Catapult & Attach Soldier if there isn't
  (bind _assoldier_ai (Utilities|Casting|CastToSoldierAI OtherActor))
  (Variables|/Game/Vive/Blueprints/AI/SoldierAI.SoldierAI_C|SetCatapult _assoldier_ai (Variables|Default|GetNextCatapult)))

(event Collision|EventHit
  (params (MyComp :type Primitive%20Component%20Object%20Reference) (Other :type Actor%20Object%20Reference) (OtherComp :type Primitive%20Component%20Object%20Reference) (bSelfMoved :type Boolean) (HitLocation :type Vector :default "0, 0, 0") (HitNormal :type Vector :default "0, 0, 0") (NormalImpulse :type Vector :default "0, 0, 0") (Hit :type Hit%20Result%20Structure%20%28by%20ref%29))
  ;[1 1 1] Destroy Catapult
  (if (Actor|ActorHasTag Other "FireArrow")
    (Variables|Default|SetIsOnFire true)))

(event EventTick
  (params (DeltaSeconds :type Float%20%28single-precision%29))
  ;[1 1 1] UpdateHealth
  (if (<= (Variables|Default|GetHealth) 0.0)
    (Actor|DestroyActor)
    (else
      (bind _ascatapult_health_bar (Utilities|Casting|CastToCatapultHealthBar (UserInterface|GetUserWidgetObject (Variables|Default|GetCatapuleHelathBarComponent))))
      (Transformation|SetWorldRotation (Variables|Default|GetCatapuleHelathBarComponent) (Math|Rotator|FindLookatRotation (Transformation|GetWorldLocation (Variables|Default|GetCatapuleHelathBarComponent)) (Transformation|GetActorLocation (Game|Player|GetPlayerPawn 0))) false false)
      (Progress|SetPercent (Variables|/Game/WidgetUI/CatapultHealthBar.CatapultHealthBar_C|GetProgressBar_143 _ascatapult_health_bar) (/ (Variables|Default|GetHealth) 1e+02))
      (if (Variables|Default|GetIsOnFire)
        (Variables|Default|SetHealth (- (Variables|Default|GetHealth) 0.05)))
      ;[1 1 1] Moving AI
      (if (Variables|Default|GetIsFull?)
        (if (Variables|Default|GetHasPosition)
          (Components|Movement|StopMovementImmediately (Variables|Character|GetCharacterMovement))
          (elif (Variables|/Game/Vive/Blueprints/AI/AiStops_Catapult.AiStops_Catapult_C|GetLastStation? (Variables|Default|GetFirstPos))
            (if (Variables|/Game/Vive/Blueprints/AI/AiAttackPosition_Catapult.AiAttackPosition_Catapult_C|GetPositionTaken (Variables|Default|GetFinalLocation))
              (AI|AIMoveTo self "0, 0, 0" (Variables|/Game/Vive/Blueprints/AI/AiAttackPosition_Catapult.AiAttackPosition_Catapult_C|GetNextPosition (Variables|Default|GetFinalLocation)) 5.0 true
                (:then
                  (Variables|Default|SetFinalLocation (Variables|/Game/Vive/Blueprints/AI/AiAttackPosition_Catapult.AiAttackPosition_Catapult_C|GetNextPosition (Variables|Default|GetFinalLocation)))))
              (else
                (AI|AIMoveTo self "0, 0, 0" (Variables|Default|GetFinalLocation) 5.0 true)))))))))

(event Collision|EventActorBeginOverlap
  (params (OtherActor :type Actor%20Object%20Reference))
  (bind _handlestring2 (Variables|Default|GetHandleString2))
  (bind _handlestring1 (Variables|Default|GetHandleString1))
  ;[1 1 1] Checking for someone manning Catapult & Attach Soldier if there isn't
  (if (Actor|ActorHasTag OtherActor "Soldier")
    (if (not (Variables|Default|GetHandleBool2))
      (if (Variables|Default|GetHandleBool1)
        (Variables|Default|SetHandleBool2 true)
        (Development|PrintString _handlestring2)
        (Transformation|AttachComponentToComponent OtherActor (Variables|Character|GetMesh) (Utilities|String|StringToName _handlestring2) "SnapToTarget" "SnapToTarget" "KeepWorld" false)
        (Variables|/Script/Engine.CharacterMovementComponent|SetMaxWalkSpeed (Variables|Character|GetCharacterMovement) 4e+02)
        (Variables|Default|SetIsFull? true)
        (AI|AIMoveTo self "0, 0, 0" (Variables|Default|GetFirstPos) 1e+01 false)
        (else
          (Variables|Default|SetHandleBool1 true)
          (Development|PrintString _handlestring1)
          (Transformation|AttachComponentToComponent OtherActor (Variables|Character|GetMesh) (Utilities|String|StringToName _handlestring1) "SnapToTarget" "SnapToTarget" "KeepWorld" false)
          (Variables|/Script/Engine.CharacterMovementComponent|SetMaxWalkSpeed (Variables|Character|GetCharacterMovement) 2e+02))))))

(fn ConstructionScript
  (Variables|Default|SetHandleBool1 false)
  (Variables|Default|SetHandleString1 "Handle1")
  (Variables|Default|SetHandleString2 "Handle2")
  (Variables|Default|SetHandleBool2 false))