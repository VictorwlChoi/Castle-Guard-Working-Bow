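; Soldier AI pawn that marches to a first stop, then heads for either a catapult to man or an attack position, and dies when hit by an arrow.
; Tick picks the route from the catapult's handle flag and a navigation path-length comparison, reissuing AIMoveTo.
; Attackers wait on the stop's LastStation flag, then walk a linked chain past taken positions.
; Overlapping an attack position or non-full catapult sets HasPosition.
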(event OnComponentBeginOverlap(CapsuleComponent)
  (params (OverlappedComponent :type Primitive%20Component%20Object%20Reference) (OtherActor :type Actor%20Object%20Reference) (OtherComp :type Primitive%20Component%20Object%20Reference) (OtherBodyIndex :type Integer) (bFromSweep :type Boolean) (SweepResult :type Hit%20Result%20Structure%20%28by%20ref%29))
  ;[1 1 1] Moving AI
  (Utilities|Casting|CastToAiAttackPosition OtherActor)
  (Variables|Default|SetHasPosition true))

(event Collision|EventHit
  (params (MyComp :type Primitive%20Component%20Object%20Reference) (Other :type Actor%20Object%20Reference) (OtherComp :type Primitive%20Component%20Object%20Reference) (bSelfMoved :type Boolean) (HitLocation :type Vector :default "0, 0, 0") (HitNormal :type Vector :default "0, 0, 0") (NormalImpulse :type Vector :default "0, 0, 0") (Hit :type Hit%20Result%20Structure%20%28by%20ref%29))
  ;[1 1 1] Death By Arrow
  (if (Actor|ActorHasTag Other "Arrow")
    (Actor|DestroyActor)))

(event EventTick
  (params (DeltaSeconds :type Float%20%28single-precision%29))
  (bind _returnvalue (Transformation|GetActorLocation))
  ;[1 1 1] Moving AI
  (if (Variables|/Game/Vive/Blueprints/AI/Catapult.Catapult_C|GetHandleBool1 (Variables|Default|GetCatapult))
    (if (not (Variables|Default|GetHasPosition)) :!label _label
      (if (Variables|/Game/Vive/Blueprints/AI/AiStops_Soldier.AiStops_Soldier_C|GetLastStation? (Variables|Default|GetFirstStop))
        (if (Variables|/Game/Vive/Blueprints/AI/AiAttackPosition.AiAttackPosition_C|GetPositionTaken (Variables|Default|GetAttackPos))
          (AI|AIMoveTo self "0, 0, 0" (Variables|/Game/Vive/Blueprints/AI/AiAttackPosition.AiAttackPosition_C|GetNextPosition (Variables|Default|GetAttackPos)) 5.0 true
            (:then
              (Variables|Default|SetAttackPos (Variables|/Game/Vive/Blueprints/AI/AiAttackPosition.AiAttackPosition_C|GetNextPosition (Variables|Default|GetAttackPos)))))
          (else
            (AI|AIMoveTo self "0, 0, 0" (Variables|Default|GetAttackPos) 5.0 true)))))
    (elif (< (.PathLength (Class|NavigationSystem|GetPathLength _returnvalue (Transformation|GetActorLocation (Variables|Default|GetFirstStop)))) (.PathLength (Class|NavigationSystem|GetPathLength _returnvalue (Transformation|GetActorLocation (Variables|Default|GetCatapult)))))
      (goto _label)
      (else
        (AI|AIMoveTo self "0, 0, 0" (Variables|Default|GetCatapult) 1e+01 false)))))

(event EventBeginPlay
  ;[1 1 1] Moving AI
  (AI|AIMoveTo self "0, 0, 0" (Variables|Default|GetFirstStop) 1e+01 false))

(event Collision|EventActorBeginOverlap
  (params (OtherActor :type Actor%20Object%20Reference))
  ;[1 1 1] Manning Catapult
  (if (Utilities|ClassIsChildOf (Utilities|GetClass OtherActor) "/Game/Vive/Blueprints/AI/Catapult.Catapult_C")
    (if (not (Variables|/Game/Vive/Blueprints/AI/Catapult.Catapult_C|GetIsFull? (Variables|Default|GetCatapult)))
      (Variables|Default|SetHasPosition true))))

(fn ConstructionScript)