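; Prototype AI battering ram that picks up overlapping actors tagged "Soldier" as carriers.
; On overlap it attaches the soldier to the first free of two handle sockets on its static mesh, tracked by a boolean per handle.
; Once the first handle is taken, Tick calls AI MoveTo every frame, though no pawn or destination is wired in.
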(event EventBeginPlay)

(event Collision|EventActorBeginOverlap
  (params (OtherActor :type Actor%20Object%20Reference))
  (bind _handlestring2 (Variables|Default|GetHandleString2))
  (bind _handlestring1 (Variables|Default|GetHandleString1))
  (if (Actor|ActorHasTag OtherActor "Soldier")
    (if (not (Variables|Default|GetHandleBool2))
      (if (Variables|Default|GetHandleBool1)
        (Variables|Default|SetHandleBool2 true)
        (Development|PrintString _handlestring2)
        (Transformation|AttachComponentToComponent OtherActor (Variables|Default|GetStaticMesh) (Utilities|String|StringToName _handlestring2) "SnapToTarget" "SnapToTarget" "KeepWorld" false)
        (else
          (Variables|Default|SetHandleBool1 true)
          (Development|PrintString _handlestring1)
          (Transformation|AttachComponentToComponent OtherActor (Variables|Default|GetStaticMesh) (Utilities|String|StringToName _handlestring1) "SnapToTarget" "SnapToTarget" "KeepWorld" false))))))

(event EventTick
  (params (DeltaSeconds :type Float%20%28single-precision%29))
  (if (Variables|Default|GetHandleBool1)
    (AI|AIMoveTo 0 "0, 0, 0" 0 5.0 true)))

(fn ConstructionScript
  (Variables|Default|SetHandleString1 "Handle1")
  (Variables|Default|SetHandleString2 "Handle2")
  (Variables|Default|SetRamIdNumber 0)
  (Variables|Default|SetHandleBool1 false)
  (Variables|Default|SetHandleBool2 false))