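; VR pawn for motion-controller archery, with a bow spawned on the left hand and arrows spawned in the right by its trigger.
; A status enum nocks the arrow when the hands meet; release then fires it, or drops it if un-nocked.
; Tick maps hand distance to draw position and rumble, and distance also sets launch speed.
; Left trigger toggles two-hand mode, which aims the bow along the line between hands.
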(event EventBeginPlay
  (CallFunction|BowSpawnandAttachtoLeftHand)
  (CallFunction|SetPrompt))

(event EventTick
  (params (DeltaSeconds :type Float%20%28single-precision%29))
  (Utilities|FlowControl|Sequence
    (:then_0
      (if (and (Utilities|Enum|Equal(Enum) (Variables|Default|Getstatus) "NewEnumerator1") (< (CallFunction|GetDistanceOfHands) 1e+01))
        (Variables|Default|Setstatus "NewEnumerator2")
        (CallFunction|ArrowAttachtoBow)))
    (:then_1
      (if (Utilities|Enum|Equal(Enum) (Variables|Default|Getstatus) "NewEnumerator2")
        (if (Variables|Default|GetTwoHandMode)
          (CallFunction|BowRotate))
        (CallFunction|ArrowUpdatePosition)))))

(event Input|KeyboardEvents|MotionControllerRightTrigger
  (params (Key :type Key%20Structure :default "AnyKey"))
  (:Pressed
    (CallFunction|ArrowSpawnandAttachtoRightHand)
    (Variables|Default|Setstatus "NewEnumerator1")
    (Rendering|SetVisibility (Variables|Default|GetVive_Control) false false)
    (Variables|Default|SetJustReleased false))
  (:Released
    (if (Utilities|Enum|Equal(Enum) (Variables|Default|Getstatus) "NewEnumerator2")
      (CallFunction|ArrowShoot)
      (else
        (CallFunction|ArrowDrop)))
    (Variables|Default|Setstatus "NewEnumerator0")
    (Game|Feedback|PlayDynamicForceFeedback (Game|GetPlayerController 0) 0.0 0.0 false false true true)
    (Rendering|SetVisibility (Variables|Default|GetVive_Control) true false)
    (Variables|Default|SetJustReleased true)))

(event Input|KeyboardEvents|MotionControllerLeftTrigger
  (params (Key :type Key%20Structure :default "AnyKey"))
  (:Pressed
    (CallFunction|ToggleMode)))

(event Custom|BowRotate
  (bind _right_hand_controller (Variables|Default|GetRight_Hand_Controller))
  (bind _left_hand_controller (Variables|Default|GetLeft_Hand_Controller))
  (bind _returnvalue (Transformation|GetWorldLocation _right_hand_controller))
  (bind _returnvalue_2 (Transformation|GetWorldLocation _left_hand_controller))
  (bind _returnvalue_3 (Class|KismetMathLibrary|GetDirectionVector _returnvalue _returnvalue_2))
  (bind _returnvalue_4 (Math|Conversions|RotationFromXVector _returnvalue_3))
  (bind (_roll _pitch _yaw) (Math|Rotator|BreakRotator _returnvalue_4))
  (Transformation|SetActorRotation (Variables|Default|Getbow) (Math|Rotator|MakeRotator _roll (+ _pitch 9e+01) _yaw)))

(event Custom|ArrowUpdatePosition
  (bind _returnvalue (CallFunction|GetDistanceOfHands))
  (bind _bow (Variables|Default|Getbow))
  (bind _returnvalue_2 (Math|Float|MapRangeClamped _returnvalue 1e+01 9e+01 3e+01 7e+01))
  (bind _attacharrowpoint (Variables|/Game/Vive/Blueprints/BP_Bow.BP_Bow_C|GetattachArrowPoint _bow))
  (bind _relativelocation (Variables|/Script/Engine.SceneComponent|GetRelativeLocation _attacharrowpoint))
  (Transformation|SetRelativeLocation (Variables|/Game/Vive/Blueprints/BP_Bow.BP_Bow_C|GetattachArrowPoint (Variables|Default|Getbow)) (Math|Vector|MakeVector _returnvalue_2 (.y _relativelocation) (.z _relativelocation)) false false)
  (Utilities|FlowControl|Sequence
    (:then_0
      (Game|Feedback|PlayDynamicForceFeedback (Game|GetPlayerController 0) (Math|Float|MapRangeClamped (CallFunction|GetDistanceOfHands) 1e+01 9e+01 0.1 0.5) 0.05 false false true true))
    (:then_1
      (Variables|Default|Setstrength (- _returnvalue_2 3e+01)))))

(event Custom|ArrowAttachToBow
  (Class|SceneComponent|Attachto (Variables|/Game/Vive/Blueprints/BP_Arrow.BP_Arrow_C|GetScene (Variables|Default|Getarrow)) (Variables|/Game/Vive/Blueprints/BP_Bow.BP_Bow_C|GetattachArrowPoint (Variables|Default|Getbow)) "" "SnapToTarget" false))

(event Custom|ArrowShoot
  (bind _arrow (Variables|Default|Getarrow))
  (bind _projectilemovement (Variables|/Game/Vive/Blueprints/BP_Arrow.BP_Arrow_C|GetProjectileMovement _arrow))
  (Class|SceneComponent|DetachfromParent (Variables|/Game/Vive/Blueprints/BP_Arrow.BP_Arrow_C|GetScene (Variables|Default|Getarrow)) true false)
  (Components|Activation|SetActive _projectilemovement true false)
  (Collision|SetActorEnableCollision _arrow true)
  (Variables|/Script/Engine.MovementComponent|SetVelocity _projectilemovement (* (Math|Vector|RotateVector "1.000000,0.000000,0.000000" (Transformation|GetWorldRotation (Variables|/Game/Vive/Blueprints/BP_Bow.BP_Bow_C|GetForwardArrow (Variables|Default|Getbow)))) (Math|Float|MapRangeClamped (CallFunction|GetDistanceOfHands) 1.5e+02 2e+02 1e+03 2e+03))))

(event Custom|ArrowDrop
  (Class|SceneComponent|DetachfromParent (Variables|/Game/Vive/Blueprints/BP_Arrow.BP_Arrow_C|GetScene (Variables|Default|Getarrow)) false true)
  (Physics|SetSimulatePhysics (Variables|/Game/Vive/Blueprints/BP_Arrow.BP_Arrow_C|GetStaticMesh (Variables|Default|Getarrow)) true))

(event Custom|SetPrompt
  (Rendering|Components|TextRender|SetText (Variables|Default|GetTextRender) (Utilities|Text|FormatText "{%s} Mode.<br>Pull trigger to toggle." (Utilities|Text|ToText(String) (Utilities|String|SelectString "Two Hands" "One Hand" (Variables|Default|GetTwoHandMode))))))

(event Custom|ToggleMode
  (Variables|Default|SetTwoHandMode (not (Variables|Default|GetTwoHandMode)))
  (CallFunction|BowResetRotation)
  (CallFunction|SetPrompt))

(event Custom|BowResetRotation
  (Transformation|SetActorRotation (Variables|Default|Getbow) (Transformation|GetWorldRotation (Variables|Default|GetLeft_Hand_Controller))))

(event Custom|BowSpawnAndAttachToLeftHand
  (bind _returnvalue (Game|SpawnActorfromClass "/Game/Vive/Blueprints/BP_Bow.BP_Bow_C" (Variables|Default|Getbow_transform) "Undefined" 0 0))
  (bind _output_get (Variables|Default|Setbow _returnvalue))
  (Class|Actor|AttachRootComponentto _output_get (Variables|Default|GetLeft_Hand_Controller) "None" "KeepRelativeOffset" true))

(event Custom|ArrowSpawnAndAttachToRightHand
  (bind _returnvalue (Game|SpawnActorfromClass "/Game/Vive/Blueprints/BP_Arrow.BP_Arrow_C" (Variables|Default|Getarrow_transform) "Undefined" 0 0))
  (bind _output_get (Variables|Default|Setarrow _returnvalue))
  (Class|SceneComponent|Attachto (Variables|/Game/Vive/Blueprints/BP_Arrow.BP_Arrow_C|GetScene _output_get) (Variables|Default|GetRight_Hand_Controller) "None" "KeepRelativeOffset" true))

(fn ConstructionScript)

(fn GetDistanceOfHands
  (return (Math|Vector|VectorLength (- (Transformation|GetWorldLocation (Variables|Default|GetRight_Hand_Controller)) (Transformation|GetWorldLocation (Variables|Default|GetLeft_Hand_Controller))))))