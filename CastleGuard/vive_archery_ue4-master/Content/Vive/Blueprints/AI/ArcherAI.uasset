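; ArcherAI is a Blueprint that moves an archer pawn along a chain of stations toward an open position.
; Each Tick without a position, it moves to the next VolumeCheck station, advancing that reference on success.
; With InFinalPosition set, it heads to FirstPos, or steps to its NextPosition if taken, updating FirstPos immediately rather than on arrival.
; HasPosition and InFinalPosition are only read here, and debug strings print which position branch runs.
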(event EventTick
  (params (DeltaSeconds :type Float%20%28single-precision%29))
  (if (not (Variables|Default|GetHasPosition))
    (if (Variables|Default|GetInFinalPosition)
      (if (Variables|/Game/Vive/Blueprints/AI/AI_Position1.AI_Position1_C|GetPositionTaken (Variables|Default|GetFirstPos))
        (Development|PrintString "true")
        (AI|AIMoveTo self "0, 0, 0" (Variables|/Game/Vive/Blueprints/AI/AI_Position1.AI_Position1_C|GetNextPosition (Variables|Default|GetFirstPos)) 5.0 false
          (:then
            (Variables|Default|SetFirstPos (Variables|/Game/Vive/Blueprints/AI/AI_Position1.AI_Position1_C|GetNextPosition (Variables|Default|GetFirstPos)))))
        (else
          (Development|PrintString "false")
          (AI|AIMoveTo self "0, 0, 0" (Variables|Default|GetFirstPos) 5.0 false)))
      (else
        (AI|AIMoveTo self "0, 0, 0" (Variables|/Game/Vive/Blueprints/AI/AI_CheckingVolume.AI_CheckingVolume_C|GetNextStation (Variables|Default|GetVolumeCheck)) 5.0 false
          (:OnSuccess
            (Variables|Default|SetVolumeCheck (Variables|/Game/Vive/Blueprints/AI/AI_CheckingVolume.AI_CheckingVolume_C|GetNextStation (Variables|Default|GetVolumeCheck)))))))))

(fn ConstructionScript)