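; AI_Position1 is a position marker that redirects ArcherAI pawns to a next position when it is occupied.
; Its Box overlap events toggle PositionTaken on begin and end, without filtering which actor overlaps.
; While that flag is set, every Tick finds all ArcherAI actors, orders each to move to NextPosition and updates its FirstPos to match.
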(event OnComponentBeginOverlap(Box)
  (params (OverlappedComponent :type Primitive%20Component%20Object%20Reference) (OtherActor :type Actor%20Object%20Reference) (OtherComp :type Primitive%20Component%20Object%20Reference) (OtherBodyIndex :type Integer) (bFromSweep :type Boolean) (SweepResult :type Hit%20Result%20Structure%20%28by%20ref%29))
  (Variables|Default|SetPositionTaken true))

(event OnComponentEndOverlap(Box)
  (params (OverlappedComponent :type Primitive%20Component%20Object%20Reference) (OtherActor :type Actor%20Object%20Reference) (OtherComp :type Primitive%20Component%20Object%20Reference) (OtherBodyIndex :type Integer))
  (Variables|Default|SetPositionTaken false))

(event EventTick
  (params (DeltaSeconds :type Float%20%28single-precision%29))
  (bind _nextposition (Variables|Default|GetNextPosition))
  (if (Variables|Default|GetPositionTaken)
    (bind _outactors (Actor|GetAllActorsOfClass "/Game/AI/ArcherAI.ArcherAI_C"))
    (for _array_element _outactors
      (AI|AIMoveTo _array_element "0, 0, 0" _nextposition 5.0 true
        (:then
          (Variables|/Game/AI/ArcherAI.ArcherAI_C|SetFirstPos _array_element _nextposition))))))

(fn ConstructionScript)